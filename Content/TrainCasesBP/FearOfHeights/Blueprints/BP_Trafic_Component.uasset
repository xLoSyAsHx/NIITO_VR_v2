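; Traffic component that drives its owning vehicle pawn along BP_SplinePawn splines by setting transforms directly.
; BeginPlay picks the closest nearby spline start, then a Tick state machine moves to it, follows the spline and randomly picks a nearby next spline at each end.
; A front box overlap finds other traffic components and triggers waiting unless they already wait, ramping speed down until clear and back up when following resumes.
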(event `self.ReceiveBeginPlay`
  ;[1 1 1] Begin Play - Choose Start and Move to it
  (bind _aspawn (cast `Pawn` (`self.GetOwner`)))
  (set `self.Vehicle Pawn` _aspawn)
  (bind _splines (`self.Get Splines In Sphere`))
  (bind _closest_spline (`self.Get Closest Spline Start` _splines))
  (bind _output_get (set `self.Current Spline To Move` _closest_spline))
  (set `self.Current Distance on Spline` 0.0)
  (`KismetSystemLibrary.Delay` 3.0)
  (`/Engine/EditorBlueprintResources/StandardMacros.IsValid` _output_get
    (:`Is Valid`
      (set `self.Current State` "NewEnumerator0"))
    (:`Is Not Valid`
      (set `self.Current State` "NewEnumerator3"))))

(event `self.ReceiveTick`
  (params (DeltaSeconds :type "Float (single-precision)"))
  (bind (_deltavector _rotator) (`self.Calculate MoveTo DeltaV and Rot`))
  (bind _speedcoef (`self.SpeedCoef`))
  (bind _speedcoef_2 (`self.SpeedCoef`))
  (bind _current_spline_to_move (`self.Current Spline To Move`))
  (set `self.Current Delta Seconds` DeltaSeconds)
  (`|ExecutionSequence`
    (:`then_0`
      (`/Engine/EditorBlueprintResources/StandardMacros.IsValid` (`self.Current Spline To Move`)
        (:`Is Valid`
          ;[1 1 1] Check For Possible Collisions With Other Vehicles
          (if (not (`self.Is Awaits Other Vehicles`))
            (bind _traffic_components (`self.Get Other VehicleTComp In Front`))
            (if (> (`KismetArrayLibrary.Array_Length` _traffic_components) 0)
              (for _array_element _traffic_components
                (if (not (`self.Is Awaits Other Vehicles` _array_element))
                  (set `self.Stored State` (`self.Current State`))
                  (set `self.Current State` "NewEnumerator4")
                  (break))))))))
    (:`then_1`
      (switch `/Game/TrainCasesBP/FearOfHeights/Blueprints/Trafic_Component_Enum` (`self.Current State`)
        (:`NewEnumerator0`
          (`|ExecutionSequence`
            (:`then_0`
              ;[1 1 1] Move To Start
              (`/Engine/EditorBlueprintResources/StandardMacros.DoOnce` false :!label _label
                (:`Completed`
                  (set `self.MoveTo_DeltaVector` _deltavector)
                  (`Actor.K2_SetActorRotation` (`self.Vehicle Pawn`) _rotator true)
                  (if (`self.Is Debug`)
                    (`KismetSystemLibrary.DrawDebugSphere` (`SplineComponent.GetLocationAtDistanceAlongSpline` (`self.Current Spline To Move`) 0.0 "World") 200.0 12 (struct :`R` 0.154355 :`G` 1.0 :`A` 1.0) 3.0)
                    (`KismetSystemLibrary.DrawDebugSphere` (`SplineComponent.GetLocationAtDistanceAlongSpline` _current_spline_to_move (`SplineComponent.GetSplineLength` _current_spline_to_move) "World") 200.0 12 (struct :`R` 0.703125 :`A` 1.0) 3.0)))))
            (:`then_1`
              (`Actor.K2_SetActorLocation` (`self.Vehicle Pawn`) (+ (`Actor.K2_GetActorLocation` (`self.Vehicle Pawn`)) (* (* (`self.MoveTo_DeltaVector`) (`self.Current Delta Seconds`)) 60.0)) false true)
              (if (`self.Is Vehicle Near Spline Point` 0)
                (set `self.Current State` "NewEnumerator1")
                (if (`self.Is Debug`)
                  (`KismetSystemLibrary.PrintString` "Move along spline")
                  (goto _label :!via `Reset`)
                  (else
                    (goto _label :!via `Reset`)))))))
        (:`NewEnumerator1`
          ;[1 1 1] Mova Along Spline
          (`self.MovaAlongSpline` _speedcoef_2)
          (if (< _speedcoef_2 1.0)
            (set `self.SpeedCoef` (+ _speedcoef_2 0.05))
            (else
              (set `self.SpeedCoef` 1.0))))
        (:`NewEnumerator2`
          ;[1 1 1] Choose Next Spline To Move To
          (bind _return (`self.Get Valid Splines Start`))
          (`|ExecutionSequence`
            (:`then_0`
              (if (`self.Is Debug`)
                (`KismetSystemLibrary.PrintString` (`KismetStringLibrary.Concat_StrStr` "Num of Founded splines:  " (`KismetStringLibrary.Conv_IntToString` (`KismetArrayLibrary.Array_Length` _return))))))
            (:`then_1`
              (if (> (`KismetArrayLibrary.Array_Length` _return) 0)
                (bind _output_get (set `self.Current Spline To Move` (`|GetArrayItem` _return (`KismetMathLibrary.RandomIntegerInRange` 0 (`KismetArrayLibrary.Array_LastIndex` _return)))))
                (bind _distance (`self.Find Distance Along Spline Closest To World Location` (`Actor.K2_GetActorLocation` (`self.Vehicle Pawn`)) _output_get))
                (set `self.Current Distance on Spline` _distance)
                (if (`self.Is Vehicle Near Spline Point` 0)
                  (set `self.Current State` "NewEnumerator1")
                  (else
                    (set `self.Current State` "NewEnumerator0")))
                (if (`self.Is Debug`)
                  (`KismetSystemLibrary.PrintString` (`|GetEnumeratorNameAsString` (`self.Current State`)) true true (struct :`G` 0.890625 :`B` 0.869189 :`A` 1.0) 5.0))
                (else
                  (set `self.Current Spline To Move` null)
                  (set `self.Current Distance on Spline` 0.0)
                  (set `self.Current State` "NewEnumerator3")
                  (if (`self.Is Debug`)
                    (`KismetSystemLibrary.PrintString` (`KismetStringLibrary.Concat_StrStr` "ERROR: Vehicle  \"" (`KismetSystemLibrary.GetObjectName` (`self.Vehicle Pawn`)) "\"  doesn't find any splines to move to") true true (struct :`R` 1.0 :`A` 1.0) 5.0)))))))
        (:`NewEnumerator4`
          ;[1 1 1] Awaits Other Vehicles to continue moving
          (bind _traffic_components_2 (`self.Get Other VehicleTComp In Front`))
          (if (== (`KismetArrayLibrary.Array_Length` _traffic_components_2) 0)
            (set `self.Current State` (`self.Stored State`))
            (else
              (`self.MovaAlongSpline` _speedcoef)
              (if (> _speedcoef 0.0)
                (set `self.SpeedCoef` (- _speedcoef 0.05))
                (else
                  (`KismetSystemLibrary.Delay` 3.0)
                  (set `self.SpeedCoef` 1.0))))))))))

(fn `Calculate MoveTo DeltaV and Rot`
  (returns (DeltaVector :type "Vector Structure") (Rotator :type "Rotator Structure"))
  (bind _returnvalue (`KismetMathLibrary.Normal` (- (`SplineComponent.GetLocationAtSplinePoint` (`self.Current Spline To Move`) 0 "World") (`Actor.K2_GetActorLocation` (`self.Vehicle Pawn`)))))
  (return (* _returnvalue (`self.Forward Speed In km/h`)) (`KismetMathLibrary.MakeRotFromX` _returnvalue)))

(fn `Find Distance Along Spline Closest To World Location`
  (params (Location :type "Vector Structure") (Spline :type "SplineComponent Object Reference"))
  (returns (Distance :type "Float (double-precision)"))
  (bind _returnvalue (`SplineComponent.FindInputKeyClosestToWorldLocation` Spline Location))
  (bind _returnvalue_2 (`KismetMathLibrary.FTrunc` _returnvalue))
  (bind _returnvalue_3 (`SplineComponent.GetDistanceAlongSplineAtSplinePoint` Spline _returnvalue_2))
  (return (+ _returnvalue_3 (* (- (`SplineComponent.GetDistanceAlongSplineAtSplinePoint` Spline (`KismetMathLibrary.FTrunc` (+ _returnvalue 1.0))) _returnvalue_3) (- _returnvalue (`KismetMathLibrary.Conv_IntToDouble` _returnvalue_2))))))

(fn `Get Closest Spline Start`
  (params (Splines :type "Array of Actor Object Reference"))
  (returns (`Closest Spline` :type "SplineComponent Object Reference"))
  (locals (ClosestSpline :type "SplineComponent Object Reference") (ClosestSplineDistance :type "Float (double-precision)" :default 10000.0))
  (for _array_element Splines
    (if (`self.Is Debug`)
      (`KismetSystemLibrary.PrintString` (`KismetSystemLibrary.GetDisplayName` _array_element)))
    (bind _asbp_spline_pawn (cast `/Game/TrainCasesBP/FearOfHeights/Blueprints/BP_SplinePawn` _array_element))
    (bind _spline (`/Game/TrainCasesBP/FearOfHeights/Blueprints/BP_SplinePawn.Spline` _asbp_spline_pawn))
    (bind _returnvalue (`KismetMathLibrary.Vector_Distance` (`SplineComponent.GetLocationAtSplinePoint` _spline 0 "World") (`Actor.K2_GetActorLocation` (`self.Vehicle Pawn`))))
    (if (< _returnvalue (`local.ClosestSplineDistance`))
      (set `local.ClosestSplineDistance` _returnvalue)
      (set `local.ClosestSpline` _spline)))
  (return (`local.ClosestSpline`)))

(fn `Get Other VehicleTComp In Front`
  (returns (`Traffic Components` :type "Array of /Game/TrainCasesBP/FearOfHeights/Blueprints/BP_Trafic_Component Object Reference"))
  (locals (`Vehicle Traffic Components` :type "Array of /Game/TrainCasesBP/FearOfHeights/Blueprints/BP_Trafic_Component Object Reference"))
  (bind _vehicle_pawn (`self.Vehicle Pawn`))
  (bind _vehiclefrontoverlapbox (`self.VehicleFrontOverlapBox`))
  (bind _returnvalue (+ (* (`Actor.GetActorForwardVector` _vehicle_pawn) 400) (`Actor.K2_GetActorLocation` _vehicle_pawn)))
  (`|ExecutionSequence`
    (:`then_0`
      (if (or (`self.Is Debug`) (`self.ShowIntersectsCheck`))
        (`KismetSystemLibrary.DrawDebugBox` _returnvalue _vehiclefrontoverlapbox (struct :`R` 1.0 :`G` 0.045922 :`A` 1.0))))
    (:`then_1`
      (bind _outactors (`KismetSystemLibrary.BoxOverlapActors` _returnvalue _vehiclefrontoverlapbox (`|MakeArray` "ObjectTypeQuery2" :!type "EObjectTypeQuery Enum") null (`|MakeArray` (`self.Vehicle Pawn`) :!type "Actor Object Reference")))
      (for _array_element _outactors
        (`KismetArrayLibrary.Array_Add` (`local.Vehicle Traffic Components`) (`Actor.GetComponentByClass` _array_element "BP_Trafic_Component_C")))
      (return (`local.Vehicle Traffic Components`)))))

(fn `Get Splines In Sphere`
  (returns (Splines :type "Array of Actor Object Reference"))
  (bind _returnvalue (`Actor.K2_GetActorLocation` (`self.Vehicle Pawn`)))
  (`|ExecutionSequence`
    (:`then_0`
      (if (`self.Is Debug`)
        (`KismetSystemLibrary.DrawDebugSphere` _returnvalue (`self.Spline Serach Sphere Radius`) 12 (struct :`R` 1.0 :`G` 1.0 :`B` 1.0 :`A` 1.0) 20.0)))
    (:`then_1`
      (bind _outactors (`KismetSystemLibrary.SphereOverlapActors` _returnvalue (`self.Spline Serach Sphere Radius`) (`|MakeArray` "ObjectTypeQuery1" :!type "EObjectTypeQuery Enum") "/Game/TrainCasesBP/FearOfHeights/Blueprints/BP_SplinePawn.BP_SplinePawn_C"))
      (return _outactors))))

(fn `Get Valid Splines Start`
  (returns (Return :type "Array of SplineComponent Object Reference"))
  (locals (`Valid Splines` :type "Array of SplineComponent Object Reference"))
  (bind _returnvalue (`Actor.K2_GetActorLocation` (`self.Vehicle Pawn`)))
  (`|ExecutionSequence`
    (:`then_0`
      (if (`self.Is Debug`)
        (`KismetSystemLibrary.DrawDebugSphere` _returnvalue (`self.Spline Serach Sphere Radius`) 12 (struct :`R` 1.0 :`G` 1.0 :`B` 1.0 :`A` 1.0) 20.0)))
    (:`then_1`
      (bind _outactors (`KismetSystemLibrary.SphereOverlapActors` _returnvalue (`self.Spline Serach Sphere Radius`) (`|MakeArray` "ObjectTypeQuery1" :!type "EObjectTypeQuery Enum") "/Game/TrainCasesBP/FearOfHeights/Blueprints/BP_SplinePawn.BP_SplinePawn_C"))
      (for _array_element _outactors
        (bind _asbp_spline_pawn (cast `/Game/TrainCasesBP/FearOfHeights/Blueprints/BP_SplinePawn` _array_element))
        (if (< (`KismetMathLibrary.Vector_Distance` (`SplineComponent.GetLocationAtSplinePoint` (`/Game/TrainCasesBP/FearOfHeights/Blueprints/BP_SplinePawn.Spline` _asbp_spline_pawn) 0 "World") (`Actor.K2_GetActorLocation` (`self.Vehicle Pawn`))) (`self.Spline Serach Sphere Radius`))
          (`KismetArrayLibrary.Array_Add` (`local.Valid Splines`) (`/Game/TrainCasesBP/FearOfHeights/Blueprints/BP_SplinePawn.Spline` _asbp_spline_pawn))))
      (return (`local.Valid Splines`)))))

(fn `Is Awaits Other Vehicles`
  (returns (ReturnValue :type Boolean))
  (return (`|EnumEquality` "NewEnumerator4" (`self.Current State`))))

(fn `Is Vehicle Near Spline Point`
  (params (`Point Index` :type Integer))
  (returns (ReturnValue :type Boolean))
  (return (< (`KismetMathLibrary.Vector_DistanceSquared` (`Actor.K2_GetActorLocation` (`self.Vehicle Pawn`)) (`SplineComponent.GetLocationAtSplinePoint` (`self.Current Spline To Move`) `Point Index` "World")) 2000.0)))

(fn `MovaAlongSpline`
  (params (`Speed Coef` :type "Float (double-precision)"))
  (bind _returnvalue (+ (`self.Current Distance on Spline`) (* `Speed Coef` (* 60.0 (* (`self.Forward Speed In km/h`) (`self.Current Delta Seconds`))))))
  (`|ExecutionSequence`
    (:`then_0`
      ;[1 1 1] Mova Along Spline
      (`Actor.K2_SetActorLocation` (`self.Vehicle Pawn`) (`SplineComponent.GetLocationAtDistanceAlongSpline` (`self.Current Spline To Move`) _returnvalue "World") false true)
      (bind _output_get (set `self.Current Distance on Spline` _returnvalue))
      (if (> _output_get (`SplineComponent.GetSplineLength` (`self.Current Spline To Move`)))
        (set `self.Current State` "NewEnumerator2")
        (if (`self.Is Debug`)
          (`KismetSystemLibrary.PrintString` (`|GetEnumeratorNameAsString` (`self.Current State`)) true true (struct :`G` 0.890625 :`B` 0.869189 :`A` 1.0) 5.0))))
    (:`then_1`
      (`Actor.K2_SetActorRotation` (`self.Vehicle Pawn`) (`SplineComponent.GetRotationAtDistanceAlongSpline` (`self.Current Spline To Move`) _returnvalue "World") true))))