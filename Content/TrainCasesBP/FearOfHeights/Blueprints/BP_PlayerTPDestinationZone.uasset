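; BP_PlayerTPDestinationZone is a player teleport destination zone marker in the Fear of Heights case.
; Its construction script colors the static mesh green for a player save zone, otherwise yellow, orange or red by Light, Medium or Hard difficulty.
; The text render shows a separate label for save zones and the difficulty enum name for the others.
; It has no active runtime logic; the event graph holds only disabled stub events.
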(fn `UserConstructionScript`
  (locals (NewLocalVar_0 :type Text :default "NSLOCTEXT(\"\", \"12B7907042D9B0D522BF4D9027332B14\", \"None\")"))
  (if (`self.Is Player Save Zone`)
    (`PrimitiveComponent.SetMaterial` (`self.StaticMesh`) 0 "/Game/TrainCasesBP/FearOfHeights/Materials/M_Green.M_Green")
    (`TextRenderComponent.K2_SetText` (`self.TextRender`) (`local.NewLocalVar_0`))
    (else
      (switch `/Game/TrainCasesBP/FearOfHeights/Blueprints/TPZoneDifficulty_Enum` (`self.Teleport Zone Difficult Type`)
        (:`NewEnumerator0`
          (`PrimitiveComponent.SetMaterial` (`self.StaticMesh`) 0 "/Game/TrainCasesBP/FearOfHeights/Materials/M_Yellow.M_Yellow"))
        (:`NewEnumerator1`
          (`PrimitiveComponent.SetMaterial` (`self.StaticMesh`) 0 "/Game/TrainCasesBP/FearOfHeights/Materials/M_Orange.M_Orange"))
        (:`NewEnumerator2`
          (`PrimitiveComponent.SetMaterial` (`self.StaticMesh`) 0 "/Game/TrainCasesBP/FearOfHeights/Materials/M_Red.M_Red")))
      (`TextRenderComponent.K2_SetText` (`self.TextRender`) (`KismetTextLibrary.Conv_StringToText` (`|GetEnumeratorNameAsString` (`self.Teleport Zone Difficult Type`)))))))