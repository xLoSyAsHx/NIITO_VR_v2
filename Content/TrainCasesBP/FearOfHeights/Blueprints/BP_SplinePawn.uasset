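; BP_SplinePawn is a spline-based Blueprint in the FearOfHeights case that visually marks a path's start and end, with no active runtime logic.
; Its construction script caches both endpoints, then adds a green cylinder at the component origin and a scaled yellow one at the end.
; It yaws an arrow by the start-to-end angle, using Y direction for sign.
; The Turn switch is empty, and point-editing fragments are disconnected.
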(fn `UserConstructionScript`
  (locals (Multiplier :type Integer :default -1) (NextPointPos :type "Vector Structure") (NextPointPosDelta :type "Vector Structure"))
  (bind _spline (`self.Spline`))
  (bind _spline_2 (`self.Spline`))
  (bind (_returnvalue_x _returnvalue_y) (`KismetMathLibrary.BreakVector` (`SplineComponent.GetLocationAtSplinePoint` (`self.Spline`) 0 "Local")))
  (bind (_returnvalue_x_2 _returnvalue_y_2) (`KismetMathLibrary.BreakVector` (`SplineComponent.GetLocationAtSplinePoint` _spline_2 (- (`SplineComponent.GetNumberOfSplinePoints` _spline_2) 1) "Local")))
  (`|ExecutionSequence`
    (:`then_0`
      ;[1 1 1] Set Start and End Spline Points Location
      (set `self.StartPointPos` (`SplineComponent.GetLocationAtSplinePoint` (`self.Spline`) 0 "Local"))
      (set `self.EndPointPos` (`SplineComponent.GetLocationAtSplinePoint` _spline (- (`SplineComponent.GetNumberOfSplinePoints` _spline) 1) "Local")))
    (:`then_1`
      ;[1 1 1] Mesh for Start Point
      (bind _returnvalue (`AddComponent|NODE_AddSplineMeshComponent-0`))
      (`StaticMeshComponent.SetStaticMesh` _returnvalue "/Game/ExternalContent/StarterContent/Shapes/Shape_Cylinder.Shape_Cylinder")
      (bind (_min _max) (`StaticMeshComponent.GetLocalBounds` _returnvalue))
      (bind _returnvalue_2 (- (.x _max) (.x _min)))
      (`SceneComponent.K2_AddLocalOffset` _returnvalue (`KismetMathLibrary.MakeVector` (/ _returnvalue_2 -2.0)) false false)
      (`PrimitiveComponent.SetMaterial` _returnvalue 0 "/Game/TrainCasesBP/FearOfHeights/Materials/M_Green.M_Green"))
    (:`then_2`
      ;[1 1 1] Mesh for End Point
      (bind _returnvalue_3 (`AddComponent|NODE_AddSplineMeshComponent-2`))
      (`StaticMeshComponent.SetStaticMesh` _returnvalue_3 "/Game/ExternalContent/StarterContent/Shapes/Shape_Cylinder.Shape_Cylinder")
      (`SceneComponent.K2_AddLocalOffset` _returnvalue_3 (+ (`KismetMathLibrary.MakeVector` (/ _returnvalue_2 -4.0)) (`self.EndPointPos`)) false false)
      (`PrimitiveComponent.SetMaterial` _returnvalue_3 0 "/Game/TrainCasesBP/FearOfHeights/Materials/M_Yellow.M_Yellow")
      (`SceneComponent.SetWorldScale3D` _returnvalue_3 (0.5 0.5 2.0))
      ;[1 1 1] Arrow
      (if (> (- _returnvalue_y_2 _returnvalue_y) 0.0)
        (set `local.Multiplier` 1))
      (`SceneComponent.K2_AddLocalRotation` (`self.Arrow`) (`KismetMathLibrary.MakeRotator` 0.0 0.0 (* (`local.Multiplier`) (`KismetMathLibrary.DegAcos` (`KismetMathLibrary.Vector_CosineAngle2D` (- (`self.EndPointPos`) (`self.StartPointPos`)) (1.0 0.0 0.0))))) false false)
      (switch `/Game/TrainCasesBP/FearOfHeights/Blueprints/Spline_Turn_Enum` (`self.Turn`)))))